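; Game instance for PlateAndPain that brings up the client's backend connection and holds the player's server-assigned identity.
; Init polls an HTTP health endpoint with growing retry delays, then passes a currently stubbed auth check before opening a WebSocket with client, level and JWT headers.
; The socket sends periodic keepalives and parses JSON messages, storing GUID and name from identity assignments; other message types are not yet handled.
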(event Custom|On%20Message
  (params (MessageString :type String))
  ;[0.15 0.15 0.15 0.5] Websocket
  (Development|PrintString "Message Received")
  (bind (_outjsonobject _returnvalue) (Class|JsonBlueprintFunctionLibrary|FromString MessageString))
  (if _returnvalue
    (bind (_outvalue _returnvalue_2) (|GetJsonField _outjsonobject "messageType"))
    (if _returnvalue_2
      (bind _outvalue_2 (|GetJsonField _outjsonobject "playerGuid"))
      (bind _outvalue_3 (|GetJsonField _outjsonobject "payload"))
      (bind _outvalue_4 (|GetJsonField _outjsonobject "requestGuid"))
      (if (Utilities|Array|ContainsItem (Utilities|Array|MakeArray "NewEnumerator23") _outvalue) ; This runs before player is in Level, which loads PPPlayerController
        (switch Utilities|FlowControl|Switch|SwitchonEN_NetworkMessageType _outvalue
          (:NewEnumerator23
            (Variables|Default|SetPlayerGuid _outvalue_2)
            (bind _outvalue_5 (|GetJsonField _outvalue_3 "playerName"))
            (Variables|Default|SetPlayerName _outvalue_5)))
        (else
          (switch Utilities|FlowControl|Switch|SwitchonEN_NetworkMessageType (.MessageType (Utilities|Struct|BreakST_NetworkWrapper (Utilities|Struct|MakeST_NetworkWrapper _outvalue _outvalue_2 _outvalue_3 _outvalue_4))))))
      (else
        (Development|PrintString "MessageType Not Found")))
    (else
      (Development|PrintString "Failure Parsing Message"))))

(event Custom|CheckAuthAndThenStartWebsocketConnection
  (Variables|Default|SetIsAuthenticated true)
  (SaveGame|LoadGamefromSlot "PlayerAuth")
  (if (and (Variables|Default|GetIsAuthenticated) (Variables|Default|GetIsServerAvailable))
    (Development|PrintString "Branch to Start Websocket" true true "(R=0.000000,G=0.660000,B=1.000000,A=1.000000)" 5.0)
    (Development|PrintString "TODO: Call Auth Verified Event Dispatcher")
    (Development|PrintString "Auth Verified" true true "(R=0.000000,G=0.660000,B=1.000000,A=1.000000)" 5.0)
    (Development|PrintString "TODO: Configure Sentry")
    (Development|PrintString "Sentry Configured" true true "(R=0.000000,G=0.660000,B=1.000000,A=1.000000)" 5.0)
    (CallFunction|SetupWebsocketConnection)
    (Development|PrintString "Websocket Connection Called" true true "(R=0.000000,G=0.660000,B=1.000000,A=1.000000)" 5.0)
    (else
      (Utilities|FlowControl|Delay 0.5) ; Wait for Player to go through auth
      (CallFunction|WaitingforPlayer))))

(event Custom|OnConnected
  (bind _websocket (Variables|Default|GetWebSocket))
  ;[0.15 0.15 0.15 0.5] Websocket
  (Variables|Default|SetIsServerConnected true)
  (Development|PrintString "Websocket connected!")
  (Class|BlueprintWebSocket|SendMessage _websocket "Client connected!")
  (Utilities|FlowControl|Delay 1e+01 :!label _label)
  (Class|BlueprintWebSocket|SendMessage _websocket "__KEEPALIVE__")
  (goto _label))

(event Custom|WaitingForPlayer
  (if (and (Variables|Default|GetIsAuthenticated) (Variables|Default|GetIsServerAvailable))
    (Development|PrintString "Branch to Start Websocket" true true "(R=0.000000,G=0.660000,B=1.000000,A=1.000000)" 5.0)
    (Development|PrintString "TODO: Call Auth Verified Event Dispatcher")
    (Development|PrintString "Auth Verified" true true "(R=0.000000,G=0.660000,B=1.000000,A=1.000000)" 5.0)
    (Development|PrintString "TODO: Configure Sentry")
    (Development|PrintString "Sentry Configured" true true "(R=0.000000,G=0.660000,B=1.000000,A=1.000000)" 5.0)
    (CallFunction|SetupWebsocketConnection)
    (Development|PrintString "Websocket Connection Called" true true "(R=0.000000,G=0.660000,B=1.000000,A=1.000000)" 5.0)
    (else
      (Utilities|FlowControl|Delay 0.5) ; Wait for Player to go through auth
      (CallFunction|WaitingforPlayer))))

(event Custom|CheckServerAvailable
  ;[0.8281 1 0] Setup
  (bind _responsecode (|SendHttpRequest (Utilities|Select :Index (Variables|Default|GetServerEnvironment) :NewEnumerator0 "http://localhost:8787/health" :NewEnumerator1 "" :NewEnumerator2 "") 0 "GET" "url")
    (:OnResponse
      _)
    (:OnError
      _))
  (if (== _responsecode 200)
    (Variables|Default|SetIsServerAvailable true)
    (Development|PrintString "TODO: Server Available Event Dispatcher")
    (CallFunction|CheckAuthandThenStartWebsocketConnection)
    (else
      (Utilities|FlowControl|Delay (Variables|Default|GetServerHealthCheckDuration))
      (Variables|Default|SetServerHealthCheckDuration (+ (Variables|Default|GetServerHealthCheckDuration) 2.0))
      (CallFunction|CheckServerAvailable))))

(event Custom|OnConnectionError
  (params (Message%20String :type String))
  ;[0.15 0.15 0.15 0.5] Websocket
  (Development|PrintString (Utilities|String|Append "Websocket Connection Error: " Message%20String) true true "(R=0.000000,G=0.660000,B=1.000000,A=1.000000)" 6.0))

(event Custom|OnClose
  (params (StatusCode :type Integer64) (Reason :type String) (bWasClean :type Boolean))
  ;[0.15 0.15 0.15 0.5] Websocket
  (Development|PrintString (Utilities|String|Append "Websocket Not Connected: " Reason)))

(event Custom|SetupWebsocketConnection
  (bind _serverenvironment (Variables|Default|GetServerEnvironment))
  ;[0.15 0.15 0.15 0.5] Websocket
  (Utilities|IsValid (Variables|Default|GetWebSocket)
    (:Is%20Valid
      (if (not (Class|BlueprintWebSocket|IsConnected (Variables|Default|GetWebSocket)))
        (Variables|Default|SetWebSocket (Class|BlueprintWebSocket|CreateWebSocket) :!label _label)
        (bind _returnvalue (Game|GetCurrentLevelName true))
        (Class|BlueprintWebSocket|SetHeaders (Variables|Default|GetWebSocket) (Utilities|Map|MakeMap "X-Client-ID" "Player" "CurrentLevelName" _returnvalue "Authorization" (Variables|Default|GetPlayerIDJWT)))
        (Utilities|FlowControl|Sequence
          (:then_0
            (EventDispatchers|BindEventtoOnMessageEvent (Variables|Default|GetWebSocket) (EventDispatchers|CreateEvent :!event Custom|On%20Message))
            (EventDispatchers|BindEventtoOnConnectedEvent (Variables|Default|GetWebSocket) (EventDispatchers|CreateEvent :!event Custom|OnConnected))
            (EventDispatchers|BindEventtoOnConnectionErrorEvent (Variables|Default|GetWebSocket) (EventDispatchers|CreateEvent :!event Custom|OnConnectionError))
            (EventDispatchers|BindEventtoOnCloseEvent (Variables|Default|GetWebSocket) (EventDispatchers|CreateEvent :!event Custom|OnClose)))
          (:then_1
            (Class|BlueprintWebSocket|Connect (Variables|Default|GetWebSocket) (Utilities|Select :Index _serverenvironment :NewEnumerator0 "ws://127.0.0.1:8787/connect" :NewEnumerator1 "" :NewEnumerator2 "") (Utilities|Select :Index _serverenvironment :NewEnumerator0 "ws" :NewEnumerator1 "wss" :NewEnumerator2 "wss"))))))
    (:Is%20Not%20Valid
      (goto _label))))

(event EventInit
  ;[0.8281 1 0] Setup
  (bind _responsecode (|SendHttpRequest (Utilities|Select :Index (Variables|Default|GetServerEnvironment) :NewEnumerator0 "http://localhost:8787/health" :NewEnumerator1 "" :NewEnumerator2 "") 0 "GET" "url")
    (:OnResponse
      _)
    (:OnError
      _))
  (if (== _responsecode 200)
    (Variables|Default|SetIsServerAvailable true)
    (Development|PrintString "TODO: Server Available Event Dispatcher")
    (CallFunction|CheckAuthandThenStartWebsocketConnection)
    (else
      (Utilities|FlowControl|Delay (Variables|Default|GetServerHealthCheckDuration))
      (Variables|Default|SetServerHealthCheckDuration (+ (Variables|Default|GetServerHealthCheckDuration) 2.0))
      (CallFunction|CheckServerAvailable))))