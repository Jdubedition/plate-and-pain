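; Monster character Blueprint for PlateAndPain, built on an MTK parent class and handling death and per-bone damage.
; On death it runs the parent logic, calls AIMonsterDied with itself, then destroys the actor after a short delay.
; The damage override scales base damage by the hit bone's multiplier from MonsterData, leaving it unchanged for unlisted bones.
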(event EventBeginPlay)

(event Collision|EventActorBeginOverlap
  (params (OtherActor :type Actor%20Object%20Reference)))

(event EventTick
  (params (DeltaSeconds :type Float%20%28single-precision%29)))

(event EventMTKonDead
  (params (KillerActor :type Actor%20Object%20Reference))
  (|CallParentFunction KillerActor)
  (Default|CallAIMonsterDied self)
  (Utilities|FlowControl|Delay 2.0)
  (Actor|DestroyActor))

(fn ConstructionScript
  (|CallParentFunction))

(fn MTKCalculateDamagePerBone
  (params (DamagedBone :type Name :default "None") (BaseDamage :type Float%20%28double-precision%29) (Hit%20Location :type Vector :default "0, 0, 0"))
  (bind _monsterdata (Variables|Default|GetMonsterData))
  (bind _damagemultiplierperbone (Variables|/Game/MonsterAi_Kit/MonsterAiKit_Core/Ai_Controllers/PDA_MonsterData.PDA_MonsterData_C|GetDamageMultiplierPerBone _monsterdata))
  (bind (_value _returnvalue) (Utilities|Map|Find _damagemultiplierperbone DamagedBone))
  (if _returnvalue
    (return (* BaseDamage _value))
    (else
      (return BaseDamage))))