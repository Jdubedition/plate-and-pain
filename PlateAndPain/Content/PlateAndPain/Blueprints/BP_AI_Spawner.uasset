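; AI spawner that fills a sphere area with monsters at BeginPlay and keeps it populated by replacing each one that dies.
; A self-calling delay event staggers the initial SpawnAmount at short random intervals.
; Each spawn traces downward from random points in SpawnSphere and places a randomly rotated monster above the hit.
; Monsters are tracked in an array, and their death event removes them and immediately spawns a replacement.
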(event Custom|AIMonsterHasDied
  (params (Monster_Ref :type Monster%20PPNBC%20Object%20Reference))
  (Utilities|IsValid Monster_Ref
    (:Is%20Valid
      (EventDispatchers|UnbindEventfromAIMonsterDied Monster_Ref (delegate Custom|AIMonsterHasDied))
      (Utilities|Array|RemoveItem (Variables|Default|GetMonstersArray) Monster_Ref)
      (CallFunction|AddAnotherMonser))))

(event Custom|AddAnotherMonser
  (bind _returnvalue (Math|Random|RandomUnitVector))
  (bind _spawnsphere (Variables|Default|GetSpawnSphere))
  (bind _returnvalue_2 (Transformation|GetWorldLocation _spawnsphere))
  (bind _returnvalue_3 (Components|Sphere|GetScaledSphereRadius _spawnsphere))
  (bind _returnvalue_4 (Math|Random|RandomFloatinRange 0.0 _returnvalue_3))
  (bind _returnvalue_5 (* _returnvalue _returnvalue_4))
  (bind _returnvalue_6 (+ _returnvalue_2 _returnvalue_5))
  (bind _outhit (Collision|LineTraceByChannel (+ _returnvalue_6 "0.000000,0.000000,1000.000000") (+ _returnvalue_6 "0.000000,0.000000,-2000.000000") "TraceTypeQuery1" false 0 "ForDuration"))
  (bind _returnvalue_7 (Game|SpawnActorfromClass "/Game/PlateAndPain/Blueprints/Monster_PPNBC.Monster_PPNBC_C" (Math|Transform|MakeTransform (+ (.Location (Collision|BreakHitResult _outhit)) "0.000000,0.000000,100.000000") (Math|Random|RandomRotator true)) "Undefined" "MultiplyWithRoot" 0 0 "Monsters" "/Game/PlateAndPain/Blueprints/PPMonsterData.PPMonsterData" 0))
  (bind _output_get (Variables|Default|SetMonster _returnvalue_7))
  (Utilities|IsValid _output_get
    (:Is%20Valid
      (EventDispatchers|BindEventtoAIMonsterDied _output_get (delegate Custom|AIMonsterHasDied)))
    (:Is%20Not%20Valid
      _))
  (Variables|/Game/PlateAndPain/Blueprints/Monster_PPNBC.Monster_PPNBC_C|SetAI_Spawner_Ref _output_get self)
  (Utilities|Array|Add (Variables|Default|GetMonstersArray) _output_get))

(event Custom|AddWithDelay
  (params (Delay :type Float%20%28double-precision%29))
  (bind _returnvalue (Math|Random|RandomUnitVector))
  (bind _spawnsphere (Variables|Default|GetSpawnSphere))
  (bind _returnvalue_2 (Transformation|GetWorldLocation _spawnsphere))
  (bind _returnvalue_3 (Components|Sphere|GetScaledSphereRadius _spawnsphere))
  (bind _returnvalue_4 (Math|Random|RandomFloatinRange 0.0 _returnvalue_3))
  (bind _returnvalue_5 (* _returnvalue _returnvalue_4))
  (bind _returnvalue_6 (+ _returnvalue_2 _returnvalue_5))
  (bind _result (Math|Integer|DecrementInt (Variables|Default|GetSpawnAmount))
    (:%20%20
      (if (> _result 0)
        (Utilities|FlowControl|Delay Delay)
        (CallFunction|AddwithDelay (Math|Random|RandomFloatinRange 0.2 1.0)))
      (bind _outhit (Collision|LineTraceByChannel (+ _returnvalue_6 "0.000000,0.000000,1000.000000") (+ _returnvalue_6 "0.000000,0.000000,-2000.000000") "TraceTypeQuery1" false 0 "ForDuration"))
      (bind _returnvalue_7 (Game|SpawnActorfromClass "/Game/PlateAndPain/Blueprints/Monster_PPNBC.Monster_PPNBC_C" (Math|Transform|MakeTransform (+ (.Location (Collision|BreakHitResult _outhit)) "0.000000,0.000000,100.000000") (Math|Random|RandomRotator true)) "Undefined" "MultiplyWithRoot" 0 0 "Monsters" "/Game/PlateAndPain/Blueprints/PPMonsterData.PPMonsterData" 0))
      (bind _output_get (Variables|Default|SetMonster _returnvalue_7))
      (Utilities|IsValid _output_get
        (:Is%20Valid
          (EventDispatchers|BindEventtoAIMonsterDied _output_get (delegate Custom|AIMonsterHasDied)))
        (:Is%20Not%20Valid
          _))
      (Variables|/Game/PlateAndPain/Blueprints/Monster_PPNBC.Monster_PPNBC_C|SetAI_Spawner_Ref _output_get self)
      (Utilities|Array|Add (Variables|Default|GetMonstersArray) _output_get))))

(event EventBeginPlay
  (CallFunction|AddwithDelay 0.0))

(fn ConstructionScript)