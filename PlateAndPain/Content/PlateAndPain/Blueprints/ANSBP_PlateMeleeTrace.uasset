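; Anim notify state that detects melee weapon hits on monsters during BP_PPThirdPersonCharacter attack animations.
; Each tick sphere-traces for pawns from the previous weapon tip position to the current socket position, stored on the character, covering the swept path.
; A per-swing hit list, cleared at begin and end, limits each actor to one hit.
; Monster_NBC hits take point damage and play a gore sound at the hit location.
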(fn ReceivedNotifyEnd
  (params (MeshComp :type Skeletal%20Mesh%20Component%20Object%20Reference) (Animation :type Anim%20Sequence%20Base%20Object%20Reference) (EventReference :type Anim%20Notify%20Event%20Reference%20Structure%20%28by%20ref%29))
  (Utilities|Array|Clear (Variables|Default|GetHitActorsThisSwing))
  (return false))

(fn ReceivedNotifyBegin
  (params (MeshComp :type Skeletal%20Mesh%20Component%20Object%20Reference) (Animation :type Anim%20Sequence%20Base%20Object%20Reference) (TotalDuration :type Float%20%28single-precision%29) (EventReference :type Anim%20Notify%20Event%20Reference%20Structure%20%28by%20ref%29))
  (Utilities|Array|Clear (Variables|Default|GetHitActorsThisSwing))
  (bind _asbp_ppthird_person_character (Utilities|Casting|CastToBP_PPThirdPersonCharacter (Components|GetOwner MeshComp)))
  (Variables|/Game/PlateAndPain/Blueprints/BP_PPThirdPersonCharacter.BP_PPThirdPersonCharacter_C|SetPreviousTipLocation _asbp_ppthird_person_character "0, 0, 0")
  (return false))

(fn ReceivedNotifyTick
  (params (MeshComp :type Skeletal%20Mesh%20Component%20Object%20Reference) (Animation :type Anim%20Sequence%20Base%20Object%20Reference) (FrameDeltaTime :type Float%20%28single-precision%29) (EventReference :type Anim%20Notify%20Event%20Reference%20Structure%20%28by%20ref%29))
  (bind _returnvalue (Components|GetOwner MeshComp))
  (bind _hitactorsthisswing (Variables|Default|GetHitActorsThisSwing))
  (bind _asbp_ppthird_person_character (Utilities|Casting|CastToBP_PPThirdPersonCharacter _returnvalue))
  (bind _outhits (Collision|MultiSphereTraceForObjects _returnvalue (select (Utilities|Operators|EqualEqual :A (Variables|/Game/PlateAndPain/Blueprints/BP_PPThirdPersonCharacter.BP_PPThirdPersonCharacter_C|GetPreviousTipLocation _asbp_ppthird_person_character)) (Transformation|GetSocketLocation (Variables|/Game/EssentialAnimation/SwordShield/Blueprint/BP_ThirdPersonCharacter.BP_ThirdPersonCharacter_C|GetUE5_Weapon _asbp_ppthird_person_character) (Variables|Default|GetTraceSocketEnd)) (Variables|/Game/PlateAndPain/Blueprints/BP_PPThirdPersonCharacter.BP_PPThirdPersonCharacter_C|GetPreviousTipLocation _asbp_ppthird_person_character)) (Transformation|GetSocketLocation (Variables|/Game/EssentialAnimation/SwordShield/Blueprint/BP_ThirdPersonCharacter.BP_ThirdPersonCharacter_C|GetUE5_Weapon _asbp_ppthird_person_character) (Variables|Default|GetTraceSocketEnd)) (Variables|Default|GetTraceRadius) (Utilities|Array|MakeArray "ObjectTypeQuery3") false (Utilities|Array|MakeArray _returnvalue) "ForDuration"))
  (for _array_element _outhits
    (Utilities|IsValid (.HitActor (Collision|BreakHitResult _array_element))
      (:Is%20Valid
        (if (not (Utilities|Array|ContainsItem _hitactorsthisswing (.HitActor (Collision|BreakHitResult _array_element))))
          (Utilities|Array|AddUnique _hitactorsthisswing (.HitActor (Collision|BreakHitResult _array_element)))
          (bind _asmonster_nbc (Utilities|Casting|CastToMonster_NBC (.HitActor (Collision|BreakHitResult _array_element))))
          (Game|Damage|ApplyPointDamage _asmonster_nbc (Variables|Default|GetDamageAmount) (* (.ImpactNormal (Collision|BreakHitResult _array_element)) (Class|KismetSystemLibrary|MakeLiteralInteger -1)) _array_element 0 _asbp_ppthird_person_character)
          (Audio|SpawnSoundatLocation _asmonster_nbc "/Game/PlateAndPain/Audio/MS_MonsterHitGore.MS_MonsterHitGore" (.Location (Collision|BreakHitResult _array_element)) "0, 0, 0" 1.0 1.0 0.0 0 0)))))
  (Variables|/Game/PlateAndPain/Blueprints/BP_PPThirdPersonCharacter.BP_PPThirdPersonCharacter_C|SetPreviousTipLocation _asbp_ppthird_person_character (Transformation|GetSocketLocation (Variables|/Game/EssentialAnimation/SwordShield/Blueprint/BP_ThirdPersonCharacter.BP_ThirdPersonCharacter_C|GetUE5_Weapon _asbp_ppthird_person_character) (Variables|Default|GetTraceSocketEnd)))
  (return false))