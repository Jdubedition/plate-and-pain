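; Actor component that plays left and right footstep sounds for the Plate and Pain third-person character without anim notifies.
; A looping timer checks each foot socket's height below the actor, its angle to the mesh forward vector and the character's speed to detect foot plants.
; Sounds spawn at the foot, gated by distance moved and a speed-dependent cooldown, though only left steps update the shared last-played time.
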(event Custom|RunFootstepCheck
  (bind _as_bp_ppthird_person_character (Variables|Default|GetAs%20BP%20PPThird%20Person%20Character))
  (bind _charactermovement (Variables|/Script/Engine.Character|GetCharacterMovement _as_bp_ppthird_person_character))
  (bind _velocity (Variables|/Script/Engine.MovementComponent|GetVelocity _charactermovement))
  (bind _returnvalue (Math|Vector|VectorLength _velocity))
  (bind _returnvalue_2 (> _returnvalue 6e+02))
  (bind _returnvalue_3 (Math|Float|SelectFloat 0.3 0.4 _returnvalue_2))
  (Variables|Default|SetLeftFootCooldown _returnvalue_3)
  (Variables|Default|SetRightFootCooldown _returnvalue_3)
  (Utilities|FlowControl|Sequence
    (:then_0
      (bind _shouldplay (CallFunction|ShouldPlayFootstep (Variables|Default|GetLeftFootSocketName)))
      (if (Math|Boolean|ANDBoolean _shouldplay (> (Math|Vector|VectorLength (- (Transformation|GetActorLocation (Variables|Default|GetAs%20BP%20PPThird%20Person%20Character)) (Variables|Default|GetPreviousRootLocation))) (Variables|Default|GetMinStepDistance)) (> (Utilities|Time|GetGameTimeinSeconds) (+ (Variables|Default|GetLastTimePlayed) (Variables|Default|GetLeftFootCooldown))))
        (Audio|SpawnSoundatLocation "/Game/PlateAndPain/Audio/PlayerLeftFootstep.PlayerLeftFootstep" (Transformation|GetSocketLocation (Variables|Default|GetUE5%20Manny) "foot_l") "0, 0, 0" 0.1 1.0 0.0 0 0)
        (Variables|Default|SetPreviousRootLocation (Transformation|GetActorLocation (Variables|Default|GetAs%20BP%20PPThird%20Person%20Character)))
        (Variables|Default|SetLastTimePlayed (Utilities|Time|GetGameTimeinSeconds))))
    (:then_1
      (bind _shouldplay_2 (CallFunction|ShouldPlayFootstep (Variables|Default|GetRightFootSocketName)))
      (if (Math|Boolean|ANDBoolean _shouldplay_2 (> (Math|Vector|VectorLength (- (Transformation|GetActorLocation (Variables|Default|GetAs%20BP%20PPThird%20Person%20Character)) (Variables|Default|GetPreviousRootLocation))) (Variables|Default|GetMinStepDistance)) (> (Utilities|Time|GetGameTimeinSeconds) (+ (Variables|Default|GetLastTimePlayed) (Variables|Default|GetRightFootCooldown))))
        (Audio|SpawnSoundatLocation "/Game/PlateAndPain/Audio/PlayerRightFootstep.PlayerRightFootstep" (Transformation|GetSocketLocation (Variables|Default|GetUE5%20Manny) "foot_r") "0, 0, 0" 0.1 1.0 0.0 0 0)
        (Variables|Default|SetPreviousRootLocation (Transformation|GetActorLocation (Variables|Default|GetAs%20BP%20PPThird%20Person%20Character)))
        (Variables|Default|SetRightFootCooldown (Utilities|Time|GetGameTimeinSeconds))))))

(event EventBeginPlay
  (bind _asbp_ppthird_person_character (Utilities|Casting|CastToBP_PPThirdPersonCharacter (Components|GetOwner)))
  (bind _output_get (Variables|Default|SetAs%20BP%20PPThird%20Person%20Character _asbp_ppthird_person_character))
  (Variables|Default|SetPreviousRootLocation (Transformation|GetActorLocation _output_get))
  (Variables|Default|SetUE5%20Manny (Variables|/Game/EssentialAnimation/SwordShield/Blueprint/BP_ThirdPersonCharacter.BP_ThirdPersonCharacter_C|GetUE5_Manny _output_get))
  (Utilities|Time|SetTimerbyEvent (delegate Custom|RunFootstepCheck) 0.05 true))

(fn ShouldPlayFootstep
  (params (SocketName :type Name))
  (bind _returnvalue (Math|Float|MakeLiteralFloat 1.8e+02))
  (bind _returnvalue_2 (Math|Trig|GetPI))
  (bind _ue5_manny (Variables|Default|GetUE5%20Manny))
  (bind _as_bp_ppthird_person_character (Variables|Default|GetAs%20BP%20PPThird%20Person%20Character))
  (bind _ue5_manny_2 (Variables|Default|GetUE5%20Manny))
  (bind _returnvalue_3 (Transformation|GetSocketLocation _ue5_manny_2 SocketName))
  (bind _returnvalue_4 (Transformation|GetActorLocation _as_bp_ppthird_person_character))
  (bind _returnvalue_5 (Transformation|GetSocketTransform _ue5_manny SocketName "RTS_World"))
  (bind _returnvalue_6 (Math|Vector|GetForwardVector _ue5_manny))
  (bind _returnvalue_7 (/ _returnvalue _returnvalue_2))
  (bind _z (Math|Vector|BreakVector _returnvalue_4))
  (bind _z_2 (Math|Vector|BreakVector _returnvalue_3))
  (bind _rotation (Math|Transform|BreakTransform _returnvalue_5))
  (bind _returnvalue_8 (Math|Vector|GetForwardVector _rotation))
  (bind _returnvalue_9 (- _z _z_2))
  (bind _returnvalue_10 (Math|Vector|DotProduct _returnvalue_8 _returnvalue_6))
  (bind _returnvalue_11 (Math|Trig|Acos(Degrees) _returnvalue_10))
  (bind _returnvalue_12 (* _returnvalue_11 _returnvalue_7))
  (if (and (> _returnvalue_9 8e+01) (< _returnvalue_9 9e+01))
    (if (and (< _returnvalue_12 9e+01) (> _returnvalue_12 8e+01))
      (if (> (Math|Vector|VectorLength (Transformation|GetVelocity (Variables|Default|GetAs%20BP%20PPThird%20Person%20Character))) 1e+02)
        (return true)))))